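; Player controller that spawns and possesses the player's pawn, handles held-click firing, and shows the death screen.
; On BeginPlay or spawnnewpawn, the authority spawns Pawn_bp above the first PlayerStart at random height, then hides Mort_widget and the cursor.
; Left mouse gates Tick into a delayed fireserver event that spawns green bullets at a fixed world-X offset from the pawn mesh.
; destroy_pawn displays Mort_widget with the cursor.
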(event Custom|destroy_pawn
  (bind _returnvalue (UserInterface|CreateWidget "/Game/ui/mort_widget.mort_widget_C" self))
  (UserInterface|Viewport|AddtoViewport _returnvalue 0)
  (Variables|Default|SetbShowMouseCursor true))

(event Custom|spawn%20new%20pawn
  ;[1 1 1] Spawn first pawn
  (Networking|SwitchHasAuthority
    (:Authority
      (bind _outactors (Actor|GetAllActorsOfClass "/Script/Engine.PlayerStart"))
      (bind _array_element (Utilities|Array|ForEachLoopwithBreak _outactors :!label _label)
        (:LoopBody
          (bind _returnvalue (Game|SpawnActorfromClass "/Game/bp/pawn_bp.pawn_bp_C" (Math|Transform|MakeTransform (+ (Transformation|GetActorLocation _array_element) (Math|Vector|MakeVector 0.0 0.0 (Math|Random|RandomFloatinRange 0.0 1e+03)))) "Undefined" self 0.0 2e+01))
          (Pawn|Possess _returnvalue)
          (goto _label Break))
        (:Completed
          (CallFunction|HideMortui))))))

(event Custom|hide%20mortui
  (bind _foundwidgets (Widget|GetAllWidgetsOfClass "/Game/ui/mort_widget.mort_widget_C" true))
  (for _array_element _foundwidgets
    (Widget|RemovefromParent _array_element)
    (Variables|Default|SetbShowMouseCursor false)))

(event Custom|fireserver_Event
  (params (val :type Transform))
  (Game|SpawnActorfromClass "/Game/bp/green_bullet_bp.green_bullet_bp_C" val "AdjustIfPossibleButAlwaysSpawn" 0 0))

(event EventBeginPlay
  ;[1 1 1] Spawn first pawn
  (Networking|SwitchHasAuthority
    (:Authority
      (bind _outactors (Actor|GetAllActorsOfClass "/Script/Engine.PlayerStart"))
      (bind _array_element (Utilities|Array|ForEachLoopwithBreak _outactors :!label _label)
        (:LoopBody
          (bind _returnvalue (Game|SpawnActorfromClass "/Game/bp/pawn_bp.pawn_bp_C" (Math|Transform|MakeTransform (+ (Transformation|GetActorLocation _array_element) (Math|Vector|MakeVector 0.0 0.0 (Math|Random|RandomFloatinRange 0.0 1e+03)))) "Undefined" self 0.0 2e+01))
          (Pawn|Possess _returnvalue)
          (goto _label Break))
        (:Completed
          (CallFunction|HideMortui))))))

(event EventTick
  (params (DeltaSeconds :type Float%20%28single-precision%29))
  ;[1 1 1] fire on left mouse click
  (Utilities|FlowControl|Gate true
    (:Exit
      (Utilities|FlowControl|Delay 0.2)
      (bind _aspawn_bp (Utilities|Casting|CastTopawn_bp (Pawn|GetControlledPawn)))
      (CallFunction|FireserverEvent (Math|Transform|MakeTransform (+ (Transformation|GetWorldLocation (Variables|/Game/bp/pawn_bp.pawn_bp_C|GetStaticMesh _aspawn_bp)) "300.000000,0.000000,0.000000") (Transformation|GetWorldRotation (Variables|/Game/bp/pawn_bp.pawn_bp_C|GetStaticMesh _aspawn_bp)))))))

(event Input|MouseEvents|LeftMouseButton
  (params (Key :type Key%20Structure :default "AnyKey"))
  ;[1 1 1] fire on left mouse click
  (:Pressed
    (Utilities|FlowControl|Gate true) ; enters at Open
  )
  (:Released
    (Utilities|FlowControl|Gate true) ; enters at Close
  ))

(fn ConstructionScript)